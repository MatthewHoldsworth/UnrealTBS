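; BP_Move is a gameplay ability that moves a TBSCharacter along a path.
; On activation it waits for a gameplay event, casts the payload's Instigator to TBSCharacter, and calls BeginMovement with the AbilityPath from that character's BP_PlayerController.
; It ends immediately after that call, without waiting for movement to finish.
; InitAbilityInfo sets Range from an Ability System Component attribute and prints it for debugging.
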(event Ability|EventActivateAbility
  (bind _payload (Ability|Tasks|WaitGameplayEvent :OptionalExternalTarget 0)
    (:EventReceived
      (bind _astbscharacter (Utilities|Casting|CastToTBSCharacter (.Instigator (Utilities|Struct|BreakGameplayEventData _payload)))
        (:then
          (Class|TBSCharacter|BeginMovement _astbscharacter (Variables|/Script/TBS.TBSPlayerController|GetAbilityPath (.AsBP%20Player%20Controller (Utilities|Casting|CastToBP_PlayerController (Pawn|GetController _astbscharacter))))))
        (:CastFailed
          (Development|PrintString "Hello")))
      (Ability|EndAbility))))

(event Ability|EventOnEndAbility
  (params (bWasCancelled :type Boolean)))

(event EventInitAbilityInfo
  (params (AbilitySystemComponent :type TBS%20Ability%20System%20Component%20Object%20Reference))
  (bind _output_get (Variables|Default|SetRange (Math|Float|Truncate (.ReturnValue (Ability|Attribute|GetFloatAttributefromAbilitySystemComponent AbilitySystemComponent "(AttributeName=\"MovementPoints\",Attribute=/Script/TBS.TBSAttributeSet:MovementPoints,AttributeOwner=\"/Script/CoreUObject.Class'/Script/TBS.TBSAttributeSet'\")")))))
  (Development|PrintString (Utilities|String|ToString(Integer) _output_get) true true "(R=0.778321,G=0.000000,B=1.000000,A=1.000000)" 2222.0))