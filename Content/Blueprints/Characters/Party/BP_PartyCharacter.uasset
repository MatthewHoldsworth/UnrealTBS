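; BP_PartyCharacter is a party character that moves freely via Enhanced Input and joins the tile grid when combat starts.
; On BeginPlay it initialises TBS ability system callbacks, grants test abilities and registers for game state combat changes.
; Entering combat claims the tile under it and shows a health bar widget; leaving releases the tile and hides the bar.
; Input also drives hold-to-look camera rotation and a test gameplay effect.
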(event Custom|CombatStateChanged_Event
  (params (InCombat :type Boolean))
  (bind _returnvalue (Transformation|GetActorLocation))
  (bind _returnvalue_2 (Class|TBSCharacter|GetEntityLocation))
  (bind _self self)
  (bind _widgetcomponent (Variables|Default|GetWidgetComponent))
  (bind _returnvalue_3 (Class|TBSBlueprintFunctionLibrary|WorldtoGridCoordinates _returnvalue))
  (bind _returnvalue_4 (Class|TBSBlueprintFunctionLibrary|GetGridManager _self))
  (bind (_x _y) (Utilities|Struct|BreakIntVector _returnvalue_3))
  (if InCombat
    (Development|PrintString (Utilities|GetDisplayName _returnvalue_4))
    (bind _returnvalue_5 (Class|GridManager|Tileat _returnvalue_4 _x _y))
    (Development|PrintString (Utilities|GetDisplayName _returnvalue_5))
    (Class|TileActor|SetOccupant _returnvalue_5 self)
    (Class|TBSCharacter|SetEntityLocation _returnvalue_5)
    (Development|PrintString (Utilities|GetDisplayName (Class|TBSCharacter|GetEntityLocation)) true true "(R=1.000000,G=0.087364,B=0.000000,A=1.000000)")
    (Rendering|SetVisibility _widgetcomponent true false)
    (bind _aswbp_health_bar (Utilities|Casting|CastToWBP_HealthBar (UserInterface|GetUserWidgetObject _widgetcomponent)))
    (Default|Setup _aswbp_health_bar self)
    (else
      (Utilities|IsValid _returnvalue_2
        (:Is%20Valid
          (Class|TileActor|SetOccupant _returnvalue_2)
          (Class|TBSCharacter|SetEntityLocation)
          (Rendering|SetVisibility (Variables|Default|GetWidgetComponent) false false))))))

(event Input|EnhancedActionEvents|EnhancedInputActionIA_Move
  (params (ActionValue :type Vector%202D%20Structure) (ElapsedSeconds :type Float%20%28double-precision%29) (TriggeredSeconds :type Float%20%28double-precision%29) (InputAction :type Input%20Action%20Object%20Reference :default "/Game/Blueprints/Input/Actions/OutOfCombat/IA_Move.IA_Move"))
  (Pawn|Input|AddMovementInput (Math|Vector|RotateVector (Math|Conversions|ToVector(Vector2D) ActionValue) (Transformation|GetActorRotation)) ElapsedSeconds false))

(event Input|EnhancedActionEvents|EnhancedInputActionIA_TESTKEY
  (params (ActionValue :type Boolean) (ElapsedSeconds :type Float%20%28double-precision%29) (TriggeredSeconds :type Float%20%28double-precision%29) (InputAction :type Input%20Action%20Object%20Reference :default "/Game/Blueprints/Input/Actions/OutOfCombat/IA_TESTKEY.IA_TESTKEY"))
  (GameplayEffects|ApplyGameplayEffectToSelf :self (Variables|Default|GetAbilitySystemComponent) :GameplayEffectClass "/Game/Blueprints/AbilitySystem/Effects/GE_TestAttributeChange.GE_TestAttributeChange_C")
  (bind _astbsability_system_component (Utilities|Casting|CastToTBSAbilitySystemComponent (Variables|Default|GetAbilitySystemComponent))))

(event Input|EnhancedActionEvents|EnhancedInputActionIA_FreeLock
  (params (ActionValue :type Boolean) (ElapsedSeconds :type Float%20%28double-precision%29) (TriggeredSeconds :type Float%20%28double-precision%29) (InputAction :type Input%20Action%20Object%20Reference :default "/Game/Blueprints/Input/Actions/OutOfCombat/IA_FreeLock.IA_FreeLock"))
  (Variables|Default|SetbFreeLock ActionValue))

(event Input|EnhancedActionEvents|EnhancedInputActionIA_ControllerXY
  (params (ActionValue :type Vector%202D%20Structure) (ElapsedSeconds :type Float%20%28double-precision%29) (TriggeredSeconds :type Float%20%28double-precision%29) (InputAction :type Input%20Action%20Object%20Reference :default "/Game/Blueprints/Input/Actions/IA_ControllerXY.IA_ControllerXY"))
  (bind (_x _y) (Math|Vector2D|BreakVector2D ActionValue))
  (Development|PrintString "MOUSEMOVE" true false "(R=1.000000,G=0.457612,B=0.000000,A=1.000000)" 0.1)
  (if (Variables|Default|GetbFreeLock)
    (Pawn|Input|AddControllerYawInput _x)
    (Pawn|Input|AddControllerPitchInput _y)))

(event EventBeginPlay
  (bind _astbsability_system_component (Utilities|Casting|CastToTBSAbilitySystemComponent (Variables|Default|GetAbilitySystemComponent)))
  (Class|TBSAbilitySystemComponent|InitialiseCallbacks _astbsability_system_component)
  (EventDispatchers|AssignCombatStateChanged (CallFunction|GetTBSGameState self) (delegate Custom|CombatStateChanged_Event))
  (GameplayAbilities|GiveAbility _astbsability_system_component "/Game/Blueprints/AbilitySystem/Abilities/BP_TestGameplayAbility.BP_TestGameplayAbility_C" 0 -1)
  (GameplayAbilities|GiveAbility _astbsability_system_component "/Game/Blueprints/AbilitySystem/Abilities/BP_TestSelfDamageAbility.BP_TestSelfDamageAbility_C" 0 -1))

(fn ConstructionScript)