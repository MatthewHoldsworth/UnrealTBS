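; BP_TestCharacter is a test character for exercising the Gameplay Ability System that turns to face the player.
; On BeginPlay it casts its ability system component to TBSAbilitySystemComponent and initialises its callbacks.
; Tick sets its yaw toward player character 0, and the R debug key applies the GE_TestDamage gameplay effect to itself.
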(event EventBeginPlay
  (bind _astbsability_system_component (Utilities|Casting|CastToTBSAbilitySystemComponent (Variables|Default|GetAbilitySystemComponent)))
  (Class|TBSAbilitySystemComponent|InitialiseCallbacks _astbsability_system_component))

(event Collision|EventActorBeginOverlap
  (params (OtherActor :type Actor%20Object%20Reference)))

(event EventTick
  (params (DeltaSeconds :type Float%20%28single-precision%29))
  (Transformation|SetActorRotation (Math|Rotator|MakeRotator 0.0 0.0 (.yaw (Math|Rotator|FindLookatRotation (Transformation|GetActorLocation) (Transformation|GetActorLocation (Game|GetPlayerCharacter 0))))) true))

(event Input|KeyboardEvents|DebugKeyR
  (params (Key :type Key%20Structure :default "None") (ActionValue :type Input%20Action%20Value%20Structure))
  (bind _abilitysystemcomponent (Variables|Default|GetAbilitySystemComponent))
  (:Pressed
    (GameplayEffects|ApplyGameplayEffectSpecToSelf _abilitysystemcomponent (GameplayEffects|MakeOutgoingSpec _abilitysystemcomponent "/Game/Blueprints/AbilitySystem/GE_TestDamage.GE_TestDamage_C" 1.0 (GameplayEffects|MakeEffectContext _abilitysystemcomponent)))))

(fn ConstructionScript)