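; Player controller for a turn-based strategy game that swaps Enhanced Input mapping contexts as the game state enters or leaves combat.
; Select highlights grid tiles within the clicked entity's MovementPoints range, or records the tile under the cursor when no entity is found.
; Execute-ability activates the selected GAS ability on the controlled pawn and sends it a gameplay event targeting the character under the cursor.
; Other inputs toggle combat and forward drag movement.
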(event Custom|OnTileHovered_Event
  (params (Tile :type Tile%20Actor%20Object%20Reference))
  (Development|PrintString "TILEHOVEREDED"))

(event Custom|CombatStateChanged_Event
  (params (InCombat :type Boolean))
  (CallFunction|SwitchControlScheme InCombat))

(event Input|EnhancedActionEvents|EnhancedInputActionIA_ChangeMode
  (params (ActionValue :type Boolean) (ElapsedSeconds :type Float%20%28double-precision%29) (TriggeredSeconds :type Float%20%28double-precision%29) (InputAction :type Input%20Action%20Object%20Reference :default "/Game/Blueprints/Input/Actions/IA_ChangeMode.IA_ChangeMode"))
  (bind _self self)
  (bind _astbsgame_state_base (CallFunction|GetTBSGameState _self))
  (if (Class|TBSGameStateBase|IsinCombat _astbsgame_state_base)
    (Class|TBSGameStateBase|ExitCombat _astbsgame_state_base)
    (else
      (Class|TBSGameStateBase|EnterCombat _astbsgame_state_base))))

(event Input|EnhancedActionEvents|EnhancedInputActionIA_DragMove
  (params (ActionValue :type Boolean) (ElapsedSeconds :type Float%20%28double-precision%29) (TriggeredSeconds :type Float%20%28double-precision%29) (InputAction :type Input%20Action%20Object%20Reference :default "/Game/Blueprints/Input/Actions/UIControls/IA_DragMove.IA_DragMove"))
  (Development|PrintString (Utilities|String|ToString(Boolean) ActionValue) true true "(R=1.000000,G=0.068094,B=0.000000,A=1.000000)")
  (Development|PrintString "DRAGGING: " true true "(R=0.000000,G=0.017494,B=1.000000,A=1.000000)")
  (Default|CallDragMove ActionValue))

(event Input|EnhancedActionEvents|EnhancedInputActionIA_Select
  (params (ActionValue :type Boolean) (ElapsedSeconds :type Float%20%28double-precision%29) (TriggeredSeconds :type Float%20%28double-precision%29) (InputAction :type Input%20Action%20Object%20Reference :default "/Game/Blueprints/Input/Actions/InCombat/IA_Select.IA_Select"))
  (bind _returnvalue (Game|GetGameMode))
  (bind _returnvalue_2 (Class|TBSPlayerController|GetEntityUnderCursor true))
  (bind _returnvalue_3 (Utilities|ToObject(Interface) _returnvalue_2))
  (bind _asbp_game_mode (Utilities|Casting|CastToBP_GameMode _returnvalue))
  (bind _gridmanager (Variables|/Script/TBS.TBSGameModeBase|GetGridManager _asbp_game_mode))
  (bind _output_get (Variables|Default|SetSelectedEntity _returnvalue_2))
  (Utilities|IsValid _returnvalue_3
    (:Is%20Valid
      (bind _returnvalue_4 (Class|GridManager|GetTilesinRange _gridmanager (Class|EntityInterface|GetEntityLocation _output_get) (Math|Float|Truncate (.currentvalue (Variables|/Script/TBS.TBSAttributeSet|GetMovementPoints (Class|TBSBlueprintFunctionLibrary|GetTBSAttributeSet (Ability|GetAbilitySystemComponent (.AsTBSCharacter (Utilities|Casting|CastToTBSCharacter _returnvalue_3)))))))))
      (Class|GridManager|SetHighlightTiles _gridmanager _returnvalue_4))
    (:Is%20Not%20Valid
      (bind _returnvalue_5 (Class|TBSPlayerController|GetTileUnderCursor))
      (Development|PrintString (Utilities|GetDisplayName _returnvalue_5) true true "(R=1.000000,G=0.061130,B=0.000000,A=1.000000)")
      (Variables|Default|SetSelectedTile _returnvalue_5))))

(event Input|EnhancedActionEvents|EnhancedInputActionIA_ExecuteAbility
  (params (ActionValue :type Boolean) (ElapsedSeconds :type Float%20%28double-precision%29) (TriggeredSeconds :type Float%20%28double-precision%29) (InputAction :type Input%20Action%20Object%20Reference :default "/Game/Blueprints/Input/Actions/InCombat/IA_ExecuteAbility.IA_ExecuteAbility"))
  (bind _returnvalue (Pawn|GetControlledPawn))
  (bind _returnvalue_2 (Ability|GetAbilitySystemComponent _returnvalue))
  (bind _astbscharacter (Utilities|Casting|CastToTBSCharacter (Class|TBSPlayerController|GetEntityUnderCursor false)))
  (Utilities|IsValid (.ReturnValue (Ability|GameplayAbility|GetGameplayAbilityfromSpecHandle _returnvalue_2 (Variables|Default|GetPlayerSelectedAbility)))
    (:Is%20Valid
      (Class|AbilitySystemComponent|TryActivateAbility _returnvalue_2 (Variables|Default|GetPlayerSelectedAbility) true)
      (Ability|SendGameplayEventtoActor :Actor _returnvalue :Payload (Utilities|Struct|MakeGameplayEventData "(TagName=\"\")" _returnvalue _astbscharacter 0 0 (GameplayEffects|MakeEffectContext _returnvalue_2) "(GameplayTags=)" "(GameplayTags=)" 0.0 (Ability|TargetData|AbilityTargetDatafromActor _astbscharacter))))))

(event EventBeginPlay
  (CallFunction|SwitchControlScheme false)
  (EventDispatchers|AssignCombatStateChanged (CallFunction|GetTBSGameState self) (delegate Custom|CombatStateChanged_Event))
  (Input|AddMappingContext (PlayerController|LocalPlayerSubsystems|GetEnhancedInputLocalPlayerSubsystem) "/Game/Blueprints/Input/IMC_UIControls.IMC_UIControls" 0 "(bIgnoreAllPressedKeysUntilRelease=True,bForceImmediately=False,bNotifyUserSettings=False)")
  (EventDispatchers|AssignOnTileHovered (Class|TBSBlueprintFunctionLibrary|GetGridManager self) (delegate Custom|OnTileHovered_Event)))

(fn ConstructionScript)

(fn SwitchControlScheme
  (params (InCombat :type Boolean))
  (bind _returnvalue (PlayerController|LocalPlayerSubsystems|GetEnhancedInputLocalPlayerSubsystem))
  (if InCombat
    (Input|RemoveMappingContext _returnvalue "/Game/Blueprints/Input/IMC_OutOfCombat.IMC_OutOfCombat" "(bIgnoreAllPressedKeysUntilRelease=True,bForceImmediately=False,bNotifyUserSettings=False)")
    (Input|AddMappingContext _returnvalue "/Game/Blueprints/Input/IMC_InCombat.IMC_InCombat" 0 "(bIgnoreAllPressedKeysUntilRelease=True,bForceImmediately=False,bNotifyUserSettings=False)")
    (else
      (Input|RemoveMappingContext _returnvalue "/Game/Blueprints/Input/IMC_InCombat.IMC_InCombat" "(bIgnoreAllPressedKeysUntilRelease=True,bForceImmediately=False,bNotifyUserSettings=False)")
      (Input|AddMappingContext _returnvalue "/Game/Blueprints/Input/IMC_OutOfCombat.IMC_OutOfCombat" 0 "(bIgnoreAllPressedKeysUntilRelease=True,bForceImmediately=False,bNotifyUserSettings=False)"))))