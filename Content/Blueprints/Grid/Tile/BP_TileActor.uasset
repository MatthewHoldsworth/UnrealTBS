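; BP_TileActor is a grid tile with a cube mesh that highlights under the cursor or on request through Highlight and UnHighlight events.
; When cursor hover begins, it reports itself to the grid manager as hovered; hover end only lowers the highlight.
; Both sources share a HighlightLevel counter, so overlapping requests stack, and its value drives the cube materials' Highlight scalar parameter.
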(event OnBeginCursorOver(CubeComponent)
  (params (TouchedComponent :type Primitive%20Component%20Object%20Reference))
  (bind _self self)
  (Class|GridManager|TileHovered (Class|TBSBlueprintFunctionLibrary|GetGridManager _self) _self)
  (bind _output_get (Variables|Default|SetHighlightLevel (+ (Variables|Default|GetHighlightLevel) 1)))
  (Rendering|Material|SetScalarParameterValueonMaterials (Variables|Default|GetCubeComponent) "Highlight" (Math|Conversions|ToFloat(Integer) _output_get)))

(event OnEndCursorOver(CubeComponent)
  (params (TouchedComponent :type Primitive%20Component%20Object%20Reference))
  (bind _output_get (Variables|Default|SetHighlightLevel (+ (Variables|Default|GetHighlightLevel) -1)))
  (Rendering|Material|SetScalarParameterValueonMaterials (Variables|Default|GetCubeComponent) "Highlight" (Math|Conversions|ToFloat(Integer) _output_get)))

(event EventBeginPlay)

(event Collision|EventActorBeginOverlap
  (params (OtherActor :type Actor%20Object%20Reference)))

(event EventTick
  (params (DeltaSeconds :type Float%20%28single-precision%29)))

(event EventHighlight
  (bind _output_get (Variables|Default|SetHighlightLevel (+ (Variables|Default|GetHighlightLevel) 1)))
  (Rendering|Material|SetScalarParameterValueonMaterials (Variables|Default|GetCubeComponent) "Highlight" (Math|Conversions|ToFloat(Integer) _output_get)))

(event EventUnHighlight
  (bind _output_get (Variables|Default|SetHighlightLevel (+ (Variables|Default|GetHighlightLevel) -1)))
  (Rendering|Material|SetScalarParameterValueonMaterials (Variables|Default|GetCubeComponent) "Highlight" (Math|Conversions|ToFloat(Integer) _output_get)))

(fn ConstructionScript)